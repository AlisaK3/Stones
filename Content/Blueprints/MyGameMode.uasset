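; Game mode that tracks elapsed seconds and handles game over when lives run out.
; While the StonePawner pawn's ButtonPressed flag is set, Tick creates Lives and TimerCount widgets each pass and uses a one-second Delay to increment TimeSec.
; When MaxLives reaches zero or below, it plays the game-over sound once and opens FirstLevel after a two-second delay.
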(event EventTick
  (params (DeltaSeconds :type Float%20%28single-precision%29))
  (Utilities|FlowControl|Sequence
    (:then_0
      (bind _asstone_pawner (Utilities|Casting|CastToStonePawner (Game|Player|GetPlayerPawn 0)))
      (if (Variables|/Game/Blueprints/StonePawner.StonePawner_C|GetButton%20Pressed _asstone_pawner)
        (bind _returnvalue (UserInterface|CreateWidget "/Game/Widgets/Lives.Lives_C"))
        (UserInterface|Viewport|AddtoViewport _returnvalue 0)
        (bind _returnvalue_2 (UserInterface|CreateWidget "/Game/Widgets/TimerCount.TimerCount_C"))
        (UserInterface|Viewport|AddtoViewport _returnvalue_2 0)
        (Variables|Default|SetTimeSec (Variables|Default|GetTimeSec))
        (Utilities|FlowControl|Delay 1.0)
        (Variables|Default|SetTimeSec (+ (Variables|Default|GetTimeSec) 1))))
    (:then_1
      (bind _output_get (Variables|Default|SetMax%20Lives (Variables|Default|GetMax%20Lives)))
      (if (<= _output_get 0)
        (Utilities|FlowControl|Sequence
          (:then_0
            (Utilities|FlowControl|Delay 2.0)
            (Game|OpenLevel(byName) "FirstLevel"))
          (:then_1
            (Utilities|FlowControl|DoOnce false
              (:Completed
                (Audio|PlaySoundatLocation "/Game/Sounds/game_over_Cue.game_over_Cue" "0, 0, 0" "0, 0, 0" 1.0 1.0 0.0 0 0 0)))))))))

(fn ConstructionScript)
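; Falling sphere actor that scores when it overlaps a cube and costs a life when it leaves a cube2.
; A timeline moves it vertically each frame at a speed set on spawn, boosted once game-mode TimeSec reaches 100.
; A catch flags StonePawner, plays effects and a widget, then adds to TimeSec and destroys the sphere.
; DoOnce-guarded misses play an error sound, decrement MaxLives and show GameOver at zero.
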(event Custom|MinusLive
  (Utilities|FlowControl|DoOnce false
    (:Completed
      (Audio|PlaySoundatLocation "/Game/Sounds/error_Cue.error_Cue" "0, 0, 0" "0, 0, 0" 1.0 1.0 0.0 0 0 0)
      (bind _asmy_game_mode (Utilities|Casting|CastToMyGameMode (Game|GetGameMode)))
      (bind _output_get (Variables|/Game/Blueprints/MyGameMode.MyGameMode_C|SetMax%20Lives _asmy_game_mode (- (Variables|/Game/Blueprints/MyGameMode.MyGameMode_C|GetMax%20Lives _asmy_game_mode) 1)))
      (if (== _output_get 0)
        (bind _returnvalue (UserInterface|CreateWidget "/Game/Widgets/GameOver.GameOver_C"))
        (UserInterface|Viewport|AddtoViewport _returnvalue 0)))))

(event Custom|ObjectSpeed
  ;[1 1 1] Falling Down
  (bind _asmy_game_mode (Utilities|Casting|CastToMyGameMode (Game|GetGameMode)))
  (if (< (Variables|/Game/Blueprints/MyGameMode.MyGameMode_C|GetTimeSec _asmy_game_mode) 100)
    (Variables|Default|SetObject%20Speed (Variables|Default|GetObject%20Speed))
    (else
      (Variables|Default|SetObject%20Speed (+ (* (/ (Variables|/Game/Blueprints/MyGameMode.MyGameMode_C|GetTimeSec _asmy_game_mode) 50) 2.0) (Variables|Default|GetObject%20Speed))))))

(event Collision|EventActorBeginOverlap
  (params (OtherActor :type Actor%20Object%20Reference))
  (bind _impact (Variables|Default|GetImpact))
  (Utilities|Casting|CastTocube OtherActor)
  (bind _asstone_pawner (Utilities|Casting|CastToStonePawner (Game|Player|GetPlayerPawn 0)))
  (Variables|/Game/Blueprints/StonePawner.StonePawner_C|SetObjectCollected _asstone_pawner true)
  (Rendering|SetVisibility (Variables|Default|GetSphere) false false)
  (Utilities|FlowControl|DoOnce false
    (:Completed
      (Audio|PlaySoundatLocation "/Game/Sounds/correct_Cue.correct_Cue" "0, 0, 0" "0, 0, 0" 1.0 1.0 0.0 0 0 0)
      (Rendering|SetVisibility _impact true false)
      (Class|PaperFlipbookComponent|SetPlaybackPositioninFrames _impact 0 false)
      (Utilities|FlowControl|Delay 0.5)
      (bind _returnvalue (UserInterface|CreateWidget "/Game/Widgets/+10.+10_C"))
      (UserInterface|Viewport|AddtoViewport _returnvalue 0)
      (Default|+counts _returnvalue)
      (Class|UserWidget|PlayAnimationForward _returnvalue 0 1.0 false))))

(event Collision|EventActorEndOverlap
  (params (OtherActor :type Actor%20Object%20Reference))
  (Utilities|FlowControl|Sequence
    (:then_0
      (Utilities|Casting|CastTocube OtherActor)
      (Variables|Default|SetCollected true)
      (Utilities|FlowControl|DoOnce false
        (:Completed
          (Utilities|FlowControl|Delay 0.2)
          (bind _asmy_game_mode (Utilities|Casting|CastToMyGameMode (Game|GetGameMode)))
          (Variables|/Game/Blueprints/MyGameMode.MyGameMode_C|SetTimeSec _asmy_game_mode (+ (Variables|/Game/Blueprints/MyGameMode.MyGameMode_C|GetTimeSec _asmy_game_mode) 10))
          (Actor|DestroyActor))))
    (:then_1
      (Utilities|Casting|CastTocube2 OtherActor)
      (Utilities|FlowControl|DoOnce false
        (:Completed
          (CallFunction|MinusLive))))))

(event EventBeginPlay
  ;[1 1 1] Falling Down
  (Rendering|SetVisibility (Variables|Default|GetImpact) false false)
  (CallFunction|ObjectSpeed)
  (Timeline|Timeline_0 Play
    (:Update
      (Transformation|AddActorLocalOffset (Math|Vector|MakeVector 0.0 0.0 (* (Variables|Default|GetObject%20Speed) (Utilities|Time|GetWorldDeltaSeconds))) false false))))

(fn ConstructionScript)